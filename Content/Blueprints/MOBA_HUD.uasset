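; MOBA HUD Blueprint that draws a logo material on screen and exposes layout data from a skill widget.
; On BeginPlay it stores all HeroCharacter actors in HeroCanSelection and creates the Skill widget without adding it to the viewport here.
; Helper functions read canvas slot positions and sizes for the five skill images and the EXP image, plus the offset position of any given widget.
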(event EventBeginPlay
  (bind _outactors (Actor|GetAllActorsOfClass "/Script/MOBA.HeroCharacter"))
  (Variables|Default|SetHeroCanSelection _outactors)
  (bind _returnvalue (UserInterface|CreateWidget "/Game/MOBA/widget/Skill.Skill_C"))
  (Variables|Default|SetSkillWidget _returnvalue))

(event Collision|EventActorBeginOverlap
  (params (OtherActor :type Actor%20Object%20Reference)))

(event EventTick
  (params (DeltaSeconds :type Float%20%28single-precision%29)))

(event EventDrawHUD
  (params (SizeX :type Integer) (SizeY :type Integer))
  (Class|HUD|DrawMaterialSimple "/Game/Blueprints/NobuLogo_Mat.NobuLogo_Mat" 0.0 0.0 518.0 1.1e+02 1.0 false))

(fn ConstructionScript)

(fn GetSkillPosition
  (params (n :type Integer))
  (bind _skillwidget (Variables|Default|GetSkillWidget))
  (bind _image_2 (Variables|/Game/MOBA/widget/Skill.Skill_C|GetImage_2 _skillwidget))
  (bind _image_3 (Variables|/Game/MOBA/widget/Skill.Skill_C|GetImage_3 _skillwidget))
  (bind _image_4 (Variables|/Game/MOBA/widget/Skill.Skill_C|GetImage_4 _skillwidget))
  (bind _image_1 (Variables|/Game/MOBA/widget/Skill.Skill_C|GetImage_1 _skillwidget))
  (bind _image_5 (Variables|/Game/MOBA/widget/Skill.Skill_C|GetImage_5 _skillwidget))
  (bind _returnvalue (Class|WidgetLayoutLibrary|SlotasCanvasSlot _image_5))
  (bind _returnvalue_2 (Class|WidgetLayoutLibrary|SlotasCanvasSlot _image_1))
  (bind _returnvalue_3 (Class|WidgetLayoutLibrary|SlotasCanvasSlot _image_2))
  (bind _returnvalue_4 (Class|WidgetLayoutLibrary|SlotasCanvasSlot _image_3))
  (bind _returnvalue_5 (Class|WidgetLayoutLibrary|SlotasCanvasSlot _image_4))
  (switch int n
    (:0
      (return (Class|CanvasPanelSlot|GetPosition _returnvalue_2) (Class|CanvasPanelSlot|GetSize _returnvalue_2)))
    (:1
      (return (Class|CanvasPanelSlot|GetPosition _returnvalue_3) (Class|CanvasPanelSlot|GetSize _returnvalue_3)))
    (:2
      (return (Class|CanvasPanelSlot|GetPosition _returnvalue_4) (Class|CanvasPanelSlot|GetSize _returnvalue_4)))
    (:3
      (return (Class|CanvasPanelSlot|GetPosition _returnvalue_5) (Class|CanvasPanelSlot|GetSize _returnvalue_5)))
    (:4
      (return (Class|CanvasPanelSlot|GetPosition _returnvalue) (Class|CanvasPanelSlot|GetSize _returnvalue)))))

(fn GetImagePosition
  (params (Widget :type Widget%20Object%20Reference))
  (bind _returnvalue (Class|WidgetLayoutLibrary|SlotasCanvasSlot Widget))
  (bind _layoutdata (Variables|/Script/UMG.CanvasPanelSlot|GetLayoutData _returnvalue))
  (bind _offsets (Utilities|Struct|BreakAnchorData _layoutdata))
  (bind (_left _top) (Utilities|Struct|BreakMargin _offsets))
  (return (Math|Vector2D|MakeVector2D _left _top)))

(fn GetExpPosition
  (bind _skillwidget (Variables|Default|GetSkillWidget))
  (bind _image_exp (Variables|/Game/MOBA/widget/Skill.Skill_C|GetImage_EXP _skillwidget))
  (bind _returnvalue (Class|WidgetLayoutLibrary|SlotasCanvasSlot _image_exp))
  (return (Class|CanvasPanelSlot|GetPosition _returnvalue) (Class|CanvasPanelSlot|GetSize _returnvalue)))