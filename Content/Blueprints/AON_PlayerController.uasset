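; Player controller that provides an RTS camera with edge scrolling and mouse-wheel zoom.
; Tick spawns RTS_Camera_90 at the first PlayerStart if missing, makes it the view target and locks the mouse to the viewport.
; Wheel input sets a target spring-arm length that Tick interpolates toward, also feeding camera rotation to SetFaceDirection.
; ZoomCurve, sampled at current arm length, scales both zoom step and per-frame pan speed, which ignores delta time.
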(event EventBeginPlay)

(event Custom|UpdateViewPosition
  (bind (_sizex _sizey) (HUD|GetViewportSize))
  (bind (_locationx _locationy) (Game|Player|GetMousePosition))
  (bind _zoomcurve (Variables|Default|GetZoomCurve))
  (bind _rts_camera (Variables|Default|GetRTS_Camera))
  (bind _rootcomponent (Variables|/Script/Engine.Actor|GetRootComponent _rts_camera))
  (bind _springarm (Variables|/Game/RTS_Camera_90.RTS_Camera_90_C|GetSpringArm _rts_camera))
  (bind _targetarmlength (Variables|/Script/Engine.SpringArmComponent|GetTargetArmLength _springarm))
  (bind _returnvalue (Math|Curves|GetFloatValue _zoomcurve _targetarmlength))
  (bind _returnvalue_2 (* _returnvalue 0.1))
  (bind _returnvalue_3 (* _returnvalue_2 -1.0))
  (Utilities|FlowControl|Sequence
    (:then_0
      (if (>= _locationx (- (Math|Conversions|ToFloat(Integer) _sizex) 3.0))
        (Transformation|AddLocalOffset _rootcomponent (Math|Vector|MakeVector 0.0 _returnvalue_2 0.0) false false)))
    (:then_1
      (if (<= _locationx 3.0)
        (Transformation|AddLocalOffset _rootcomponent (Math|Vector|MakeVector 0.0 _returnvalue_3 0.0) false false)))
    (:then_2
      (if (>= _locationy (- (Math|Conversions|ToFloat(Integer) _sizey) 3.0))
        (Transformation|AddLocalOffset _rootcomponent (Math|Vector|MakeVector _returnvalue_3 0.0 0.0) false false)))
    (:then_3
      (if (<= _locationy 3.0)
        (Transformation|AddLocalOffset _rootcomponent (Math|Vector|MakeVector _returnvalue_2 0.0 0.0) false false)))))

(event EventTick
  (params (DeltaSeconds :type Float%20%28single-precision%29))
  (Utilities|IsValid (Variables|Default|GetRTS_Camera)
    (:Is%20Valid
      _)
    (:Is%20Not%20Valid
      (bind _outactors (Actor|GetAllActorsOfClass "/Script/Engine.PlayerStart"))
      (bind _returnvalue (Game|SpawnActorfromClass "/Game/RTS_Camera_90.RTS_Camera_90_C" (Math|Conversions|ToTransform(Vector) (Transformation|GetActorLocation (Utilities|Array|Get(acopy) _outactors))) "Undefined" 0 0))
      (Variables|Default|SetRTS_Camera _returnvalue)
      (Game|Player|SetViewTargetwithBlend (Variables|Default|GetRTS_Camera) 0.0 "VTBlend_Linear" 0.0 false)
      (Input|SetInputModeGameandUI 0 0 "LockAlways" true)))
  (CallFunction|UpdateViewPosition)
  (Variables|/Script/Engine.SpringArmComponent|SetTargetArmLength (Variables|/Game/RTS_Camera_90.RTS_Camera_90_C|GetSpringArm (Variables|Default|GetRTS_Camera)) (Math|Interpolation|FInterpTo (Variables|/Script/Engine.SpringArmComponent|GetTargetArmLength (Variables|/Game/RTS_Camera_90.RTS_Camera_90_C|GetSpringArm (Variables|Default|GetRTS_Camera))) (Variables|Default|GetCamBoomLength) DeltaSeconds 3.0))
  (Class|DamageEffect|SetFaceDirection (Transformation|GetWorldRotation (Variables|/Game/RTS_Camera_90.RTS_Camera_90_C|GetCamera (Variables|Default|GetRTS_Camera)))))

(event Input|MouseEvents|MouseWheelUp
  (params (Key :type Key%20Structure))
  (bind _rts_camera (Variables|Default|GetRTS_Camera))
  (bind _springarm (Variables|/Game/RTS_Camera_90.RTS_Camera_90_C|GetSpringArm _rts_camera))
  (bind _targetarmlength (Variables|/Script/Engine.SpringArmComponent|GetTargetArmLength _springarm))
  (:Pressed
    (Variables|Default|SetCamBoomLength (- _targetarmlength (* (Math|Curves|GetFloatValue (Variables|Default|GetZoomCurve) _targetarmlength) 1.0)))))

(event Input|MouseEvents|MouseWheelDown
  (params (Key :type Key%20Structure))
  (bind _rts_camera (Variables|Default|GetRTS_Camera))
  (bind _springarm (Variables|/Game/RTS_Camera_90.RTS_Camera_90_C|GetSpringArm _rts_camera))
  (bind _targetarmlength (Variables|/Script/Engine.SpringArmComponent|GetTargetArmLength _springarm))
  (:Pressed
    (Variables|Default|SetCamBoomLength (+ _targetarmlength (* (Math|Curves|GetFloatValue (Variables|Default|GetZoomCurve) _targetarmlength) 1.0)))))

(fn ConstructionScript)